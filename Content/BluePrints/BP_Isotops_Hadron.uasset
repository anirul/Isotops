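; Hadron actor for an isotopes game or simulation, representing a single particle such as a proton or neutron.
; Setting its particle type stores the value and swaps the material to red for protons or white for neutrons; Alpha only prints "Not Implemented".
; A getter exposes the type, and a velocity setter overwrites the physics linear velocity through ProjectileMovement.
; Event graph and construction script hold no logic.
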(event `self.ReceiveBeginPlay`)

(event `self.ReceiveActorBeginOverlap`
  (params (OtherActor :type "Actor Object Reference")))

(event `self.ReceiveTick`
  (params (DeltaSeconds :type "Float (single-precision)")))

(fn `Get_Particule_Type`
  (returns (NewParam :type "/Game/Enums/ENUM_Isotops_Particule_type Enum"))
  (return (`self.Particule_Type`)))

(fn `Set_Particule_Type`
  (params (NewParam :type "/Game/Enums/ENUM_Isotops_Particule_type Enum" :default "NewEnumerator0"))
  (bind _output_get (set `self.Particule_Type` NewParam))
  (switch `/Game/Enums/ENUM_Isotops_Particule_type` _output_get
    (:`NewEnumerator2`
      (`PrimitiveComponent.SetMaterial` 0 "/Game/Materials/MAT_Isotops_Red.MAT_Isotops_Red"))
    (:`NewEnumerator3`
      (`PrimitiveComponent.SetMaterial` 0 "/Game/Materials/MAT_Isotops_White.MAT_Isotops_White"))
    (:`NewEnumerator4`
      (`KismetSystemLibrary.PrintString` "Not Implemented" true true (struct :`R` 1.0 :`G` 0.033789 :`A` 1.0)))))

(fn `Set_Velocity`
  (params (NewVelocity :type "Object.Vector Structure"))
  (`PrimitiveComponent.SetPhysicsLinearVelocity` (`self.ProjectileMovement`) NewVelocity false "None"))

(fn `UserConstructionScript`)