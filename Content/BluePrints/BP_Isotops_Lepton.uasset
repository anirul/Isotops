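; BP_Isotops_Lepton is a lepton projectile, either an electron or a positron, with a particle system as its visual.
; SetParticuleType stores the type and tints the particle color to match, while SetVelocityVector overrides the linear velocity through ProjectileMovement.
; Each tick, once the particle system is 5000 units or more from the world origin, it calls ApplyDamage with type-specific damage and no visible target, then destroys itself.
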(event `self.ReceiveBeginPlay`)

(event `self.ReceiveActorBeginOverlap`
  (params (OtherActor :type "Actor Object Reference")))

(event `self.ReceiveTick`
  (params (DeltaSeconds :type "Float (single-precision)"))
  ;[1 1 1] Delete if too far and create damage
  (if (>= (`KismetMathLibrary.VSize` (`SceneComponent.K2_GetComponentLocation` (`self.Particule_System`))) 5000.0)
    (switch `/Game/Enums/ENUM_Isotops_Particule_type` (`self.Particule_Type`)
      (:`NewEnumerator0`
        (`GameplayStatics.ApplyDamage` null (`self.Electron_Damage`)))
      (:`NewEnumerator1`
        (`GameplayStatics.ApplyDamage` null (`self.Positron_Damage`))))
    (`self.K2_DestroyActor`)))

(fn `Get_Particule_Type`
  (returns (NewParam :type "/Game/Enums/ENUM_Isotops_Particule_type Enum"))
  (return (`self.Particule_Type`)))

(fn `Set_Particule_Type`
  (params (NewParam :type "/Game/Enums/ENUM_Isotops_Particule_type Enum" :default "NewEnumerator0"))
  (bind _particule_system (`self.Particule_System`))
  (bind _output_get (set `self.Particule_Type` NewParam))
  (switch `/Game/Enums/ENUM_Isotops_Particule_type` _output_get
    (:`NewEnumerator0`
      (`ParticleSystemComponent.SetVectorParameter` _particule_system "Particle_Color_Param" (`self.Electron_Color`)))
    (:`NewEnumerator1`
      (`ParticleSystemComponent.SetVectorParameter` _particule_system "Particle_Color_Param" (`self.Positron_Color`)))))

(fn `Set_Velocity_Vector`
  (params (Velocity :type "Object.Vector Structure"))
  (`PrimitiveComponent.SetPhysicsLinearVelocity` (`self.ProjectileMovement`) Velocity false "None"))

(fn `UserConstructionScript`)