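; BP_Isotops_Game_Mode is the game mode for an isotopes game that rations protons and neutrons through two recharge meters.
; Both meters start empty and fill on Tick at a shared Increase rate, clamped between zero and one.
; GetProton and GetNeutron return true and reset their meter only when it is full, otherwise false, acting as independent cooldown gates.
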(event `self.ReceiveBeginPlay`
  (set `self.NeutronReady` 0.0)
  (set `self.ProtonReady` 0.0))

(event `self.ReceiveTick`
  (params (DeltaSeconds :type "Float (single-precision)"))
  (bind _returnvalue (* DeltaSeconds (`self.Increase`)))
  (set `self.ProtonReady` (`KismetMathLibrary.FClamp` (+ _returnvalue (`self.ProtonReady`))))
  (set `self.NeutronReady` (`KismetMathLibrary.FClamp` (+ (`self.NeutronReady`) _returnvalue))))

(fn `GetNeutron`
  (returns (Valid :type Boolean))
  (if (== (`self.NeutronReady`) 1.0)
    (set `self.NeutronReady` 0.0)
    (return true)
    (else
      (return false))))

(fn `GetProton`
  (returns (Valid :type Boolean))
  (if (== (`self.ProtonReady`) 1.0)
    (set `self.ProtonReady` 0.0)
    (return true)
    (else
      (return false))))

(fn `UserConstructionScript`)