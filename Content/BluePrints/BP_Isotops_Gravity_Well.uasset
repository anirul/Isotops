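; Gravity well actor that gathers hadrons into an atomic nucleus, simulating isotope identity and radioactive decay while tracking the player's radiation dose.
; Overlaps update proton and neutron counts, which set the element, half-life and lifetime.
; Tick pulls particles inward with jitter and half-life-scaled attraction, then pushes state to the pawn UI.
; Expired atoms decay by converting or ejecting nucleons, adding dose that heals gradually and resets the well at full.
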(event `self.ReceiveBeginPlay`
  ;[1 1 1] Get input from controler
  (`self.EnableInput` (`GameplayStatics.GetPlayerController` 0))
  (set `self.Cummulative_Time` 0.0)
  (`self.Update_Atom`))

(event `self.ReceiveActorBeginOverlap`
  (params (OtherActor :type "Actor Object Reference"))
  ;[1 1 1] Enter or Exit Gravity Well
  (bind _asbp_isotops_hadron (cast `/Game/BluePrints/BP_Isotops_Hadron` OtherActor))
  (`KismetArrayLibrary.Array_Add` (`self.Particle_List`) _asbp_isotops_hadron)
  ;[1 1 1] Count Protons / Neutrons
  (bind _newparam (`/Game/BluePrints/BP_Isotops_Hadron.Get_Particule_Type` _asbp_isotops_hadron))
  (switch `/Game/Enums/ENUM_Isotops_Particule_type` _newparam
    (:`NewEnumerator2`
      (set `self.NB_Proton` (+ (`self.NB_Proton`) 1)))
    (:`NewEnumerator3`
      (set `self.NB_Neutron` (+ (`self.NB_Neutron`) 1))))
  (`self.Update_Atom` :!label _label))

(event `self.ReceiveActorEndOverlap`
  (params (OtherActor :type "Actor Object Reference"))
  ;[1 1 1] Enter or Exit Gravity Well
  (bind _asbp_isotops_hadron (cast `/Game/BluePrints/BP_Isotops_Hadron` OtherActor))
  (`KismetArrayLibrary.Array_RemoveItem` (`self.Particle_List`) _asbp_isotops_hadron)
  ;[1 1 1] Count Protons / Neutrons
  (bind _newparam (`/Game/BluePrints/BP_Isotops_Hadron.Get_Particule_Type` _asbp_isotops_hadron))
  (switch `/Game/Enums/ENUM_Isotops_Particule_type` _newparam
    (:`NewEnumerator2`
      (set `self.NB_Proton` (- (`self.NB_Proton`) 1))
      (goto _label))
    (:`NewEnumerator3`
      (set `self.NB_Neutron` (- (`self.NB_Neutron`) 1))
      (goto _label))))

(event `self.ReceiveTick`
  (params (DeltaSeconds :type "Float (single-precision)"))
  ;[1 1 1] Change Physic (attract particule)
  (for _array_element (`self.Particle_List`)
    (`/Game/BluePrints/BP_Isotops_Hadron.Set_Velocity` _array_element (* (+ (- (`SceneComponent.K2_GetComponentLocation` (`self.Gravity_Well`)) (`self.K2_GetActorLocation` _array_element)) (`KismetMathLibrary.RandomUnitVector`)) (`self.Particule_Attraction`))))
  (`self.Decay_Atom` DeltaSeconds)
  (`self.Stability` (`self.Half_Life`))
  ;[1 1 1] Healing
  (bind _output_get (set `self.Radiation_Dose` (- (`self.Radiation_Dose`) (* (`self.Heal_Per_Second`) DeltaSeconds))))
  ;[1 1 1] Death condition
  (if (>= _output_get 1.0)
    (`self.Reset_Gravity_Well`))
  (`self.Send_Update_UI`))

(event `InputAction|Reset debug`
  (params (Key :type "Key Structure"))
  ;[1 1 1] Reset state
  (:`Pressed`
    (`/Engine/EditorBlueprintResources/StandardMacros.DoOnce` false :!label _label_2
      (:`Completed`
        (`self.Reset_Gravity_Well`))))
  (:`Released`
    (goto _label_2 :!via `Reset`)))

(fn `Debug_Print`
  ;[1 1 1] Debug
  (`KismetSystemLibrary.PrintString` (`KismetTextLibrary.Conv_TextToString` (`|FormatText` "Protons {NBProton} - Neutrons {NBNeutron}" (`KismetTextLibrary.Conv_IntToText` (`self.NB_Proton`)) (`KismetTextLibrary.Conv_IntToText` (`self.NB_Neutron`))))))

(fn `Decay_Atom`
  (params (DeltaTime :type "Float (double-precision)"))
  ;[1 1 1] Update cummulative time
  (set `self.Cummulative_Time` (+ DeltaTime (`self.Cummulative_Time`)))
  ;[1 1 1] Time for decay
  (if (not (>= (- (`self.Life`) (`KismetMathLibrary.Exp` (`self.Cummulative_Time`))) 0.0))
    ;[1 1 1] Debug in case decay
    (`KismetSystemLibrary.PrintString` (`KismetTextLibrary.Conv_TextToString` (`|FormatText` "Decay p{Protons} n{Neutrons}" (`KismetTextLibrary.Conv_IntToText` (`self.NB_Proton`)) (`KismetTextLibrary.Conv_IntToText` (`self.NB_Neutron`)))) false true (struct :`R` 1.0 :`G` 0.007827 :`A` 1.0))
    ;[1 1 1] Decay
    (set `self.Decay_Mode` (`NucleusModel.Decay` (`self.NB_Proton`) (`self.NB_Neutron`) (`KismetMathLibrary.RandomFloat`)))
    (for _array_element (`self.Decay_Mode`)
      (bind (_type _protons _neutrons) (break `DecayMode` _array_element))
      (switch `EDecayType` _type
        (:`Bplus`
          (`self.Spawn_EC_Decay` :!label _label))
        (:`Bminus`
          (`self.Spawn_Beta_Decay`))
        (:`EC`
          (goto _label))
        (:`Eplus`
          (goto _label))
        (:`Nucleon`
          (for _ (range 1 (+ _protons 1))
            (`self.Spawn_Proton_Decay`))
          (for _ (range 1 (+ _neutrons 1))
            (`self.Spawn_Neutron_Decay`))))
      (`self.Update_Atom`)
      ;[1 1 1] debug
      (`KismetSystemLibrary.PrintString` (`KismetTextLibrary.Conv_TextToString` (`|FormatText` "Nucleon Ejection p:{protons} n:{neutrons} size{size}" (`KismetTextLibrary.Conv_IntToText` _protons) (`KismetTextLibrary.Conv_IntToText` _neutrons) (`KismetTextLibrary.Conv_IntToText` (`KismetArrayLibrary.Array_Length` (`self.Decay_Mode`))))) false true (struct :`R` 0.636787 :`B` 1.0 :`A` 1.0)))))

(fn `Reset_Gravity_Well`
  (bind _particle_list (`self.Particle_List`))
  (set `self.Radiation_Dose` 0.0)
  (set `self.Cummulative_Time` 0.0)
  (set `self.Element_Symbol` "Null")
  (while (> (`KismetArrayLibrary.Array_Length` _particle_list) 0)
    (`self.K2_DestroyActor` (`|GetArrayItem` _particle_list))))

(fn `Send_Update_UI`
  ;[1 1 1] Update UI
  (bind _asbp_isotops_pawn (cast `/Game/BluePrints/BP_Isotops_Pawn` (`GameplayStatics.GetPlayerPawn` 0)))
  (`/Game/BluePrints/BP_Isotops_Pawn.Update_UI` _asbp_isotops_pawn (`self.Element_Symbol`) (`self.Element_Name`) (`self.Element_Description`) (`self.NB_Proton`) (`self.NB_Neutron`) (`self.Radiation_Dose`)))

(fn `Spawn_Beta_Decay`
  (bind _nb_neutron (`self.NB_Neutron`))
  (bind _particule_location (`self.Particule_Location`))
  (bind _returnvalue (- _particule_location (`SceneComponent.K2_GetComponentLocation` (`self.Gravity_Well`))))
  ;[1 1 1] Check if decay possible and decrease the numbers
  (if (== _nb_neutron 0)
    (`KismetSystemLibrary.PrintString` "Error Cannot beta decay" true true (struct :`R` 1.0 :`A` 1.0))
    (else
      (set `self.NB_Neutron` (- _nb_neutron 1))
      (set `self.NB_Proton` (+ (`self.NB_Proton`) 1))
      ;[1 1 1] Search for a Neutron to decay into Proton
      (for _array_element (`self.Particle_List`)
        (set `self.Particule_Location` (`self.K2_GetActorLocation` _array_element))
        (switch `/Game/Enums/ENUM_Isotops_Particule_type` (`/Game/BluePrints/BP_Isotops_Hadron.Particule_Type` _array_element)
          (:`NewEnumerator3`
            (`/Game/BluePrints/BP_Isotops_Hadron.Set_Particule_Type` _array_element "NewEnumerator2")
            (break))))
      ;[1 1 1] Spawn a Beta-
      (bind _returnvalue_2 (`|SpawnActorFromClass` "/Game/BluePrints/BP_Isotops_Lepton.BP_Isotops_Lepton_C" (`KismetMathLibrary.MakeTransform` _particule_location (`KismetMathLibrary.Conv_VectorToRotator` _returnvalue)) "AdjustIfPossibleButDontSpawnIfColliding" "OverrideRootScale" null null))
      (`/Game/BluePrints/BP_Isotops_Lepton.Set_Velocity_Vector` _returnvalue_2 (* _returnvalue 100.0))
      (`/Game/BluePrints/BP_Isotops_Lepton.Set_Particule_Type` _returnvalue_2 "NewEnumerator0")
      ;[1 1 1] Update Radiation Dose
      (set `self.Radiation_Dose` (+ (`self.Radiation_Dose`) (`self.Electron_Dose`))))))

(fn `Spawn_EC_Decay`
  (bind _nb_proton (`self.NB_Proton`))
  (bind _particule_location (`self.Particule_Location`))
  (bind _returnvalue (- _particule_location (`SceneComponent.K2_GetComponentLocation` (`self.Gravity_Well`))))
  ;[1 1 1] Check if decay possible and decrease the numbers
  (if (== _nb_proton 0)
    (`KismetSystemLibrary.PrintString` "Error Cannot EC decay" true true (struct :`R` 1.0 :`A` 1.0))
    (else
      (set `self.NB_Neutron` (+ (`self.NB_Neutron`) 1))
      (set `self.NB_Proton` (- _nb_proton 1))
      ;[1 1 1] Search for a Neutron to decay into Proton
      (for _array_element (`self.Particle_List`)
        (set `self.Particule_Location` (`self.K2_GetActorLocation` _array_element))
        (switch `/Game/Enums/ENUM_Isotops_Particule_type` (`/Game/BluePrints/BP_Isotops_Hadron.Particule_Type` _array_element)
          (:`NewEnumerator2`
            (`/Game/BluePrints/BP_Isotops_Hadron.Set_Particule_Type` _array_element "NewEnumerator3")
            (break))))
      ;[1 1 1] Spawn a Beta+
      (bind _returnvalue_2 (`|SpawnActorFromClass` "/Game/BluePrints/BP_Isotops_Lepton.BP_Isotops_Lepton_C" (`KismetMathLibrary.MakeTransform` _particule_location (`KismetMathLibrary.Conv_VectorToRotator` _returnvalue)) "AdjustIfPossibleButDontSpawnIfColliding" "OverrideRootScale" null null))
      (`/Game/BluePrints/BP_Isotops_Lepton.Set_Velocity_Vector` _returnvalue_2 (* _returnvalue 100.0))
      (`/Game/BluePrints/BP_Isotops_Lepton.Set_Particule_Type` _returnvalue_2 "NewEnumerator1")
      ;[1 1 1] Update Radiation Dose
      (set `self.Radiation_Dose` (+ (`self.Radiation_Dose`) (`self.Positron_Dose`))))))

(fn `Spawn_Neutron_Decay`
  (bind _particle_list (`self.Particle_List`))
  (bind _max_neutron (`self.Max_Neutron`))
  ;[1 1 1] Check if neutron left
  (if (== (`self.NB_Neutron`) 0)
    (`KismetSystemLibrary.PrintString` "Cannot Neutron Decay" true true (struct :`R` 1.0 :`A` 1.0))
    (else
      ;[1 1 1] Get the farthest neutron from the center
      (set `self.Max_Distance` 0.0)
      (for _array_element _particle_list
        (bind _newparam (`/Game/BluePrints/BP_Isotops_Hadron.Get_Particule_Type` _array_element))
        (switch `/Game/Enums/ENUM_Isotops_Particule_type` _newparam
          (:`NewEnumerator3`
            (bind _returnvalue (- (`self.K2_GetActorLocation` _array_element) (`SceneComponent.K2_GetComponentLocation`)))
            (bind _returnvalue_2 (`KismetMathLibrary.VSize` _returnvalue))
            (if (> _returnvalue_2 (`self.Max_Distance`))
              (set `self.Max_Neutron` _array_element)
              (set `self.Max_Distance` _returnvalue_2)))))
      ;[1 1 1] Remove it
      (`/Game/BluePrints/BP_Isotops_Hadron.Set_Velocity` _max_neutron (* _returnvalue (`self.Ejection_Speed`)))
      (`KismetArrayLibrary.Array_RemoveItem` _particle_list _max_neutron)
      ;[1 1 1] Update Radiation Dose
      (set `self.Radiation_Dose` (+ (`self.Radiation_Dose`) (`self.Neutron_Dose`))))))

(fn `Spawn_Proton_Decay`
  (bind _particle_list (`self.Particle_List`))
  (bind _max_proton (`self.Max_Proton`))
  ;[1 1 1] Check if neutron left
  (if (== (`self.NB_Proton`) 0)
    (`KismetSystemLibrary.PrintString` "Cannot Proton Decay" true true (struct :`R` 1.0 :`A` 1.0))
    (else
      ;[1 1 1] Get the farthest neutron from the center
      (set `self.Max_Distance` 0.0)
      (for _array_element _particle_list
        (bind _newparam (`/Game/BluePrints/BP_Isotops_Hadron.Get_Particule_Type` _array_element))
        (switch `/Game/Enums/ENUM_Isotops_Particule_type` _newparam
          (:`NewEnumerator2`
            (bind _returnvalue (- (`self.K2_GetActorLocation` _array_element) (`SceneComponent.K2_GetComponentLocation`)))
            (bind _returnvalue_2 (`KismetMathLibrary.VSize` _returnvalue))
            (if (> _returnvalue_2 (`self.Max_Distance`))
              (set `self.Max_Proton` _array_element)
              (set `self.Max_Distance` _returnvalue_2)))))
      ;[1 1 1] Remove it
      (`/Game/BluePrints/BP_Isotops_Hadron.Set_Velocity` _max_proton (* _returnvalue (`self.Ejection_Speed`)))
      (`KismetArrayLibrary.Array_RemoveItem` _particle_list _max_proton)
      ;[1 1 1] Update Radiation Dose
      (set `self.Radiation_Dose` (+ (`self.Radiation_Dose`) (`self.Proton_Dose`))))))

(fn `Stability`
  (params (Half_Life :type "Float (double-precision)"))
  (bind _returnvalue (/ 100.0 Half_Life))
  (if (> _returnvalue 1.0)
    (set `self.Particule_Attraction` 50.0)
    (elif (< _returnvalue 0.0)
      (set `self.Particule_Attraction` 1.0)
      (else
        (set `self.Particule_Attraction` (`KismetMathLibrary.Lerp` 1.0 50.0 _returnvalue))))))

(fn `Update_Atom`
  (bind (_symbol _element _description _halflife _life) (break `Nucleon` (`NucleusModel.Create` (`self.NB_Proton`) (`self.NB_Neutron`) (`KismetMathLibrary.RandomFloat`))))
  ;[1 1 1] Get Nucleon Type
  (set `self.Element_Symbol` _symbol)
  (set `self.Element_Name` _element)
  (set `self.Element_Description` _description)
  (set `self.Half_Life` _halflife)
  (set `self.Life` (+ _life (`self.Grace_Time`)))
  (set `self.Cummulative_Time` 0.0))

(fn `UserConstructionScript`
  (`self.Reset_Gravity_Well`))