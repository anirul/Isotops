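; BP_Isotops_Pawn is the player pawn that owns the on-screen UI for an isotope-themed game.
; On BeginPlay it creates a BP_Game_UI widget, stores it as GameUI and adds it to the viewport.
; Its UpdateUI function copies element symbol, name, description, proton and neutron counts and radiation dose straight into that widget's variables.
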(event `self.ReceiveBeginPlay`
  (bind _returnvalue (`|CreateWidget` "/Game/BluePrints/BP_Game_UI.BP_Game_UI_C"))
  (bind _output_get (set `self.Game_UI` _returnvalue))
  (`UserWidget.AddToViewport` _output_get 0))

(fn `Update_UI`
  (params (`Element Symbol` :type String) (`Element Name` :type String) (`Element Description` :type String) (NB_Protons :type Integer) (NB_Neutrons :type Integer) (Radiation_Dose :type "Float (double-precision)"))
  (bind _game_ui (`self.Game_UI`))
  (set `/Game/BluePrints/BP_Game_UI.Element_Symbol` `Element Symbol` _game_ui)
  (set `/Game/BluePrints/BP_Game_UI.Element_Name` `Element Name` _game_ui)
  (set `/Game/BluePrints/BP_Game_UI.Element_Description` `Element Description` _game_ui)
  (set `/Game/BluePrints/BP_Game_UI.Nb_Protons` NB_Protons _game_ui)
  (set `/Game/BluePrints/BP_Game_UI.Nb_Neutrons` NB_Neutrons _game_ui)
  (set `/Game/BluePrints/BP_Game_UI.Radiation_Dose` Radiation_Dose _game_ui))

(fn `UserConstructionScript`)